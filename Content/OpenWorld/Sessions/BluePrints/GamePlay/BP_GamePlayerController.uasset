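; Gameplay player controller that sets up the local player's HUD and game-only input, then forwards begin-play to the possessed third-person character.
; Possess triggers this multicast-style setup, reusing an existing HUD widget when valid.
; Helper events re-enable pawn input and route respawn requests to the game mode.
; Debug keys 5 and 6 switch all BP_Npc1 AI into fight mode via blackboard or kill them.
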(event Custom|RespawnAfterDeath
  (bind _asbp_game_game_mode (Utilities|Casting|CastToBP_Game_GameMode (Game|GetGameMode)))
  (Default|RespawnAfterDeath _asbp_game_game_mode self))

(event Custom|MC_BeginPlay
  (if (Pawn|IsLocalPlayerController)
    (Viewport|RemoveAllWidgets)
    (CallFunction|UIShowIngameHUD)
    (Input|SetInputModeGameOnly self false)
    (Variables|Default|SetbShowMouseCursor false)
    (bind _asbp_third_person_character (Utilities|Casting|CastToBP_ThirdPersonCharacter (Pawn|GetControlledPawn)))
    (Default|MCBeginPlay _asbp_third_person_character)
    (else
      (Development|PrintString "playercontroller not local player"))))

(event Custom|EnableAllInput
  (Input|EnableInput (Pawn|GetControlledPawn) self)
  (Development|PrintString "gameplayercontroller Enable Input"))

(event EventBeginPlay
  ;[1 1 1] For Editor when not playing menu. Delete when playing regular
)

(event EventPossess
  (params (PossessedPawn :type Pawn%20Object%20Reference))
  (CallFunction|MCBeginPlay))

(event Input|KeyboardEvents|5
  (params (Key :type Key%20Structure :default "None"))
  (:Pressed
    (Development|PrintString "Lets Get Ready To rumble")
    (bind _outactors (Actor|GetAllActorsOfClass "/Game/OpenWorld/Sessions/BluePrints/GamePlay/AI/BP_Npc1.BP_Npc1_C"))
    (for _array_element _outactors
      (bind _asaic_behavior (Utilities|Casting|CastToAIC_Behavior (Pawn|GetController _array_element)))
      (AI|Components|Blackboard|SetValueasBool (AI|GetBlackboard _asaic_behavior) (Utilities|Name|MakeLiteralName "FightMode") true))))

(event Input|KeyboardEvents|6
  (params (Key :type Key%20Structure :default "None"))
  (:Pressed
    (bind _outactors (Actor|GetAllActorsOfClass "/Game/OpenWorld/Sessions/BluePrints/GamePlay/AI/BP_Npc1.BP_Npc1_C"))
    (for _array_element _outactors
      (Default|Die _array_element "NewEnumerator0"))))

(fn ConstructionScript)

(fn UIShowIngameHUD
  (Variables|Default|GetWB_PlayedHUD
    (:then
      _)
    (:else
      (bind _returnvalue (UserInterface|CreateWidget "/Game/OpenWorld/Sessions/Widgets/WB_HeadsupDisplay.WB_HeadsupDisplay_C" self))
      (Variables|Default|SetWB_PlayedHUD _returnvalue)))
  (UserInterface|Viewport|AddtoViewport (Variables|Default|GetWB_PlayedHUD) 0)
  (return))