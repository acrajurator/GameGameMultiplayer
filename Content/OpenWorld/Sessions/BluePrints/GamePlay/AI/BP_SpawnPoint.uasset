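; Spawn point actor that, on the server, keeps an area populated with AiTest NPCs.
; BeginPlay spawns SpawnAmount pawns, then a looping timer adds one whenever ActivePawns falls below that count.
; Each NPC spawns at a random point inside the Bound component, receives a reference to this spawn point and joins ActivePawns.
; A downward ground trace runs per spawn, but its result is unused.
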(event Custom|SpawnNPCs
  (for _index (range 1 (Variables|Default|GetSpawn%20Amount))
    (CallFunction|SpawnCharacter))
  (Utilities|Time|SetTimerbyFunctionName 0 "RespawnCharacter" (Variables|Default|GetTimeToRespawn) true))

(event EventBeginPlay
  (Networking|SwitchHasAuthority
    (:Authority
      (CallFunction|SpawnNPCs))))

(fn ConstructionScript)

(fn SpawnCharacter
  (bind _bound (Variables|Default|GetBound))
  (bind (_origin _boxextent) (Collision|GetComponentBounds _bound))
  (bind _returnvalue (Math|Random|RandomPointinBoundingBox _origin _boxextent))
  (bind (_x _y _z) (Math|Vector|BreakVector _returnvalue))
  (bind _returnvalue_2 (+ _z 1e+04))
  (bind _returnvalue_3 (Math|Vector|MakeVector _x _y _returnvalue_2))
  (bind _outhit (Collision|LineTraceForObjects _returnvalue_3 (+ _returnvalue_3 (* (* (Transformation|GetActorUpVector) -1) 1.5e+04)) (Utilities|Array|MakeArray "ObjectTypeQuery1") false 0 "None"))
  (bind _returnvalue_4 (AI|SpawnAIFromClass "/Game/OpenWorld/Sessions/BluePrints/GamePlay/AI/AiTest.AiTest_C" 0 _returnvalue (Math|Rotator|MakeRotator 0.0 0.0 (Math|Random|RandomFloat)) false 0))
  (bind _asai_test (Utilities|Casting|CastToAiTest _returnvalue_4))
  (Variables|/Game/OpenWorld/Sessions/BluePrints/GamePlay/AI/AiTest.AiTest_C|SetSpawnPoint _asai_test self)
  (Utilities|Array|Add (Variables|Default|GetActivePawns) _returnvalue_4))

(fn RespawnCharacter
  (if (< (Utilities|Array|Length (Variables|Default|GetActivePawns)) (Variables|Default|GetSpawn%20Amount))
    (CallFunction|SpawnCharacter)))