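; Server-side NPC spawn point that populates a bounds volume with BP_Npc1 AI while a BP_Slime is within LoadedDistance.
; Spawns use random points (the line trace result is unused) and receive a patrol path, team, team tint and spawner reference.
; A looping respawn timer tops up from the ActivePawns count.
; A 10-second timer sets Active by slime distance, destroying tracked pawns when inactive without clearing the array.
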(event Custom|SpawnNPCs
  (for _index (range 1 (Variables|Default|GetSpawn%20Amount))
    (CallFunction|SpawnCharacter))
  (Utilities|Time|SetTimerbyFunctionName 0 "RespawnCharacter" (Variables|Default|GetTimeToRespawn) true))

(event Custom|Despawn
  (Utilities|Time|SetTimerbyFunctionName 0 "DespawnSpawner" 1e+01 true))

(event EventBeginPlay
  (Networking|SwitchHasAuthority
    (:Authority
      (CallFunction|SpawnNPCs)
      (CallFunction|DeSpawn))))

(fn ConstructionScript)

(fn SpawnCharacter
  (bind _bound (Variables|Default|GetBound))
  (bind (_origin _boxextent) (Collision|GetComponentBounds _bound))
  (bind _returnvalue (Math|Random|RandomPointinBoundingBox _origin _boxextent))
  (bind (_x _y _z) (Math|Vector|BreakVector _returnvalue))
  (bind _returnvalue_2 (+ _z 1e+04))
  (bind _returnvalue_3 (Math|Vector|MakeVector _x _y _returnvalue_2))
  (if (Variables|Default|GetActive)
    (bind _outhit (Collision|LineTraceForObjects _returnvalue_3 (+ _returnvalue_3 (* (* (Transformation|GetActorUpVector) -1) 1.5e+04)) (Utilities|Array|MakeArray "ObjectTypeQuery1") false 0 "None"))
    (bind _returnvalue_4 (AI|SpawnAIFromClass "/Game/OpenWorld/Sessions/BluePrints/GamePlay/AI/BP_Npc1.BP_Npc1_C" "/Game/OpenWorld/Sessions/BluePrints/GamePlay/AI/BehaviorTree/BT_NPC.BT_NPC" _returnvalue (Math|Rotator|MakeRotator 0.0 0.0 (Math|Random|RandomFloat)) false 0))
    (bind _asbp_npc_1 (Utilities|Casting|CastToBP_Npc1 _returnvalue_4))
    (Variables|/Game/OpenWorld/Sessions/BluePrints/GamePlay/AI/BP_Npc1.BP_Npc1_C|SetPatrolPath _asbp_npc_1 (Variables|Default|GetPatrolPath))
    (switch int (Variables|Default|GetTeam)
      (:Default
        _)
      (:0
        _)
      (:1
        (bind _returnvalue_5 (Rendering|Material|CreateDynamicMaterialInstance (Variables|/Script/Engine.Character|GetMesh _asbp_npc_1) 0 "/Game/OpenWorld/Sessions/BluePrints/GamePlay/AI/Npc02.Npc02" "None" :!class /Script/Engine.PrimitiveComponent))
        (Rendering|Material|SetVectorParameterValue _returnvalue_5 "Tint" (Utilities|Struct|MakeLinearColor 1.0 0.0 0.0 1.0) :!class /Script/Engine.MaterialInstanceDynamic))
      (:2
        (bind _returnvalue_6 (Rendering|Material|CreateDynamicMaterialInstance (Variables|/Script/Engine.Character|GetMesh _asbp_npc_1) 0 "/Game/OpenWorld/Sessions/BluePrints/GamePlay/AI/Npc02.Npc02" "None" :!class /Script/Engine.PrimitiveComponent))
        (Rendering|Material|SetVectorParameterValue _returnvalue_6 "Tint" (Utilities|Struct|MakeLinearColor 0.0 1.0 0.0 1.0) :!class /Script/Engine.MaterialInstanceDynamic))
      (:3
        (bind _returnvalue_7 (Rendering|Material|CreateDynamicMaterialInstance (Variables|/Script/Engine.Character|GetMesh _asbp_npc_1) 0 "/Game/OpenWorld/Sessions/BluePrints/GamePlay/AI/Npc02.Npc02" "None" :!class /Script/Engine.PrimitiveComponent))
        (Rendering|Material|SetVectorParameterValue _returnvalue_7 "Tint" (Utilities|Struct|MakeLinearColor 0.0 0.0 1.0 1.0) :!class /Script/Engine.MaterialInstanceDynamic)))
    (Variables|/Game/ThirdPerson/Blueprints/BP_CharacterParent.BP_CharacterParent_C|SetTeam _asbp_npc_1 (Variables|Default|GetTeam))
    (Variables|/Game/OpenWorld/Sessions/BluePrints/GamePlay/AI/BP_Npc1.BP_Npc1_C|SetSpawnPoint _asbp_npc_1 self)
    (Utilities|Array|Add (Variables|Default|GetActivePawns) _returnvalue_4)))

(fn RespawnCharacter
  (for _index (range (Utilities|Array|Length (Variables|Default|GetActivePawns)) (Variables|Default|GetSpawn%20Amount))
    (CallFunction|SpawnCharacter)))

(fn DespawnSpawner
  (bind _outactors (Actor|GetAllActorsOfClass "/Game/OpenWorld/Sessions/BluePrints/GamePlay/Slime/BP_Slime.BP_Slime_C"))
  (if (>= (Utilities|Array|Length _outactors) 1)
    (for _array_element _outactors
      (if (< (Math|Vector|Distance(Vector) (Transformation|GetActorLocation _array_element) (Transformation|GetActorLocation self)) (LocalVariables|GetLcl_PlayerDistance))
        (LocalVariables|SetLcl_PlayerDistance (Math|Vector|Distance(Vector) (Transformation|GetActorLocation _array_element) (Transformation|GetActorLocation self)))))
    (if (< (LocalVariables|GetLcl_PlayerDistance) (Variables|Default|GetLoadedDistance))
      (Variables|Default|SetActive true)
      (else
        (Variables|Default|SetActive false)
        (CallFunction|DespawnAll)))
    (else
      (Variables|Default|SetActive false)
      (CallFunction|DespawnAll))))

(fn DespawnAll
  (bind _activepawns (Variables|Default|GetActivePawns))
  (if (> (Utilities|Array|Length _activepawns) 0)
    (for _array_element _activepawns
      (Utilities|IsValid _array_element
        (:Is%20Valid
          (Actor|DestroyActor _array_element))))
    (return)))