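; Sword-wielding melee NPC character for a networked game that hunts living players on other teams.
; FindEnemy picks the player with the fewest AI attackers via a shared counter, passes it to AIC_Behavior, and MoveToPlayer re-chases it.
; While its damage flag is set, a per-tick blade sphere trace damages enemies through interfaces.
; TakeDamage computes hit direction, then triggers stun reactions or death montages, with a separate event for ragdolling body and sword.
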(event Custom|OnAISpawned
  (bind (_isvalidplayerfound _newenemy) (CallFunction|FindEnemy false :!label _label))
  (if _isvalidplayerfound
    (CallFunction|SetTargetPlayer _newenemy)
    (else
      (Utilities|FlowControl|Delay 0.5)
      (goto _label))))

(event Custom|MoveToPlayer
  (bind _self self)
  (bind _returnvalue (Transformation|GetActorRotation _self))
  (if (Variables|Default|GetIsAlive)
    (bind _movementresult (AI|AIMoveTo self "0, 0, 0" (Variables|Default|GetTargetPlayer) 8e+01 false)
      (:OnSuccess
        _)
      (:OnFail
        _))
    (switch Utilities|FlowControl|Switch|SwitchonEPathFollowingResult _movementresult
      (:Success
        (Transformation|SetActorRotation _self (Math|Rotator|MakeRotator (.roll _returnvalue) (.pitch _returnvalue) (+ (.Yaw (Math|Rotator|BreakRotator (Math|Rotator|FindLookatRotation (Transformation|GetWorldLocation (Variables|Character|GetMesh _self)) (Transformation|GetActorLocation (Variables|Default|GetTargetPlayer))))) 3e+01)) :!label _label)
        (Utilities|FlowControl|Delay 0.2)
        (bind _targetplayer (Variables|Default|GetTargetPlayer)
          (:then
            (if (Variables|/Game/ThirdPerson/Blueprints/BP_CharacterParent.BP_CharacterParent_C|GetIsAlive _targetplayer)
              (CallFunction|MovetoPlayer)
              (else
                (Variables|Default|SetTargetPlayer 0 :!label _label_2)
                (CallFunction|OnAISpawned))))
          (:else
            (goto _label_2))))
      (:Blocked
        (goto _label))
      (:OffPath
        (goto _label))
      (:Aborted
        (Development|PrintString "npc aborted"))
      (:Invalid
        (goto _label)))))

(event Custom|GetBlocked
  (CallFunction|MCStopCurrentMontage)
  (CallFunction|PlayBlockedAnim)
  (Animation|Montage|PlayMontage (Variables|Character|GetMesh) "/Game/Combat/SK_GetHit2.SK_GetHit2"
    (:then
      (Variables|Default|SetIsStunned true))
    (:OnCompleted
      (Variables|Default|SetIsStunned false :!label _label))
    (:OnBlendOut
      (goto _label))
    (:OnInterrupted
      (goto _label))))

(event Custom|PlayBlockedAnim
  (Animation|Montage|PlayMontage (Variables|Character|GetMesh) "/Game/Combat/SK_GetHit2.SK_GetHit2"))

(event Custom|Die
  (params (DamageDirection :type Enum_DamageDirection%20Enum :default "NewEnumerator0"))
  (bind _mesh (Variables|Character|GetMesh))
  (bind _targetplayer (Variables|Default|GetTargetPlayer))
  (Variables|/Script/Engine.SkeletalMeshComponent|SetKinematicBonesUpdateType _mesh "SkipSimulatingBones")
  (Variables|/Script/Engine.SkinnedMeshComponent|SetVisibilityBasedAnimTickOption _mesh "AlwaysTickPoseAndRefreshBones")
  (bind _as_aic_behavior (Variables|Default|GetAs%20AIC%20Behavior)
    (:then
      (Pawn|UnPossess _as_aic_behavior))
    (:else
      _))
  (Variables|Default|SetCanAttack false)
  (Utilities|IsValid _targetplayer
    (:Is%20Valid
      (Math|Integer|DecrementInt (Variables|/Game/ThirdPerson/Blueprints/BP_CharacterParent.BP_CharacterParent_C|GetNrOfAIAttacker _targetplayer)
        (:%20%20
          _)))
    (:Is%20Not%20Valid
      _))
  (CallFunction|MCPlayDeathMontage DamageDirection))

(event Custom|MC_PlayDeathMontage
  (params (DamageDirection :type Enum_DamageDirection%20Enum :default "NewEnumerator0"))
  (bind _deathmontage (CallFunction|GetDeathMontage DamageDirection))
  (Animation|Montage|PlayMontage (Variables|Character|GetMesh) _deathmontage))

(event Custom|StartRagdoll
  (bind _returnvalue (Utilities|Name|MakeLiteralName "root"))
  (bind _mesh (Variables|Character|GetMesh))
  (bind _sword (Variables|Default|GetSword))
  (bind _charactermovement (Variables|Character|GetCharacterMovement))
  (bind _returnvalue_2 (Pawn|Components|CharacterMovement|GetLastUpdateVelocity _charactermovement))
  (Collision|SetCollisionEnabled _sword "PhysicsOnly")
  (Collision|SetCollisionResponsetoChannel _sword "ECC_WorldStatic" "ECR_Block")
  (Physics|SetSimulatePhysics _sword true)
  (Collision|SetCollisionResponsetoChannel (Variables|Default|GetCapsuleComponent) "ECC_Pawn" "ECR_Overlap")
  (Collision|SetCollisionProfileName _mesh "Ragdoll" true :!class /Script/Engine.PrimitiveComponent)
  (Class|SkeletalMeshComponent|SetAllBodiesBelowSimulatePhysics _mesh _returnvalue true true)
  (Physics|AddImpulse _mesh (+ _returnvalue_2 (* (Math|Vector|Normalize _returnvalue_2) 400)) _returnvalue true)
  (if (Networking|IsServer)
    (Components|Movement|StopMovementImmediately (Variables|Character|GetCharacterMovement))
    (Class|SkeletalMeshComponent|SetAnimClass _mesh)
    (Components|Tick|SetComponentTickEnabled (Variables|Character|GetCharacterMovement) false)
    (Components|DestroyComponent (Variables|Character|GetCharacterMovement))
    (Components|Tick|SetComponentTickEnabled (Variables|Default|GetSword) false)
    (Variables|Default|Setragdoll true)))

(event Custom|MC_RemoveClientTrigger
  (if (not (Networking|IsServer))
    (Actor|Tick|SetActorTickEnabled false)))

(event Custom|MC_StopCurrentMontage
  (Animation|StopAnimMontage 0))

(event Custom|MC_PlayAttackMontage
  (params (MontageToPlay :type Anim%20Montage%20Object%20Reference))
  (Animation|Montage|PlayMontage (Variables|Character|GetMesh) MontageToPlay
    (:OnBlendOut
      (if (Networking|IsServer)
        (bind _result (Math|Integer|IncrementInt (Variables|Default|GetMeleeAnimIndex))
          (:%20%20
            (if (>= _result (Utilities|Array|Length (Variables|Default|GetAllAttackAnim)))
              (Variables|Default|SetMeleeAnimIndex 0))))))))

(event Custom|GetHit
  (params (MontageToPlay :type Anim%20Montage%20Object%20Reference) (Location :type Vector) (Normal :type Vector))
  (Niagara|SpawnSystematLocation "/Game/Combat/Effects/NS_Blood.NS_Blood" Location (Math|Conversions|RotationFromXVector Normal) "100.000000,100.000000,100.000000")
  (CallFunction|MCStopCurrentMontage)
  (Animation|Montage|PlayMontage (Variables|Character|GetMesh) MontageToPlay
    (:then
      (Variables|Default|SetIsStunned true))
    (:OnCompleted
      (Variables|Default|SetIsStunned false :!label _label))
    (:OnBlendOut
      (goto _label))
    (:OnInterrupted
      (goto _label))))

(event EventTick
  (params (DeltaSeconds :type Float%20%28single-precision%29))
  (CallFunction|MeleeTrace))

(event EventMeleeAttack
  (CallFunction|MCPlayAttackMontage "/Game/Characters/Mannequins/Animations/Manny/attack.attack"))

(event EventDestroyed
  (bind _self self)
  (bind _targetplayer (Variables|Default|GetTargetPlayer))
  (Networking|SwitchHasAuthority
    (:Authority
      (bind _spawnpoint (Variables|Default|GetSpawnPoint)
        (:then
          (if (Utilities|Array|ContainsItem (Variables|/Game/OpenWorld/Sessions/BluePrints/GamePlay/AI/BP_SpawnPoint1.BP_SpawnPoint1_C|GetActivePawns _spawnpoint) _self)
            (Utilities|Array|RemoveItem (Variables|/Game/OpenWorld/Sessions/BluePrints/GamePlay/AI/BP_SpawnPoint1.BP_SpawnPoint1_C|GetActivePawns _spawnpoint) _self)))
        (:else
          _))
      (Utilities|IsValid _targetplayer
        (:Is%20Valid
          (Math|Integer|DecrementInt (Variables|/Game/ThirdPerson/Blueprints/BP_CharacterParent.BP_CharacterParent_C|GetNrOfAIAttacker _targetplayer)))))))

(event EventPossessed
  (params (NewController :type Controller%20Object%20Reference))
  (bind _asaic_behavior (Utilities|Casting|CastToAIC_Behavior NewController))
  (Variables|Default|SetAs%20AIC%20Behavior _asaic_behavior)
  (Utilities|FlowControl|Delay 5.0))

(event EventDeadBody
  (if (Variables|Default|Getragdoll)
    (Actor|DestroyActor)))

(fn ConstructionScript)

(fn FindEnemy
  (params (FindClosestEnemy :type Boolean))
  (bind _outactors (Actor|GetAllActorsOfClass "/Game/ThirdPerson/Blueprints/BP_CharacterParent.BP_CharacterParent_C"))
  (LocalVariables|SetLcl_AllPlayer _outactors)
  (bind _arrayelement (Utilities|Array|ReverseforEachLoop (LocalVariables|GetLcl_AllPlayer))
    (:LoopBody
      (if (or (not (Variables|/Game/ThirdPerson/Blueprints/BP_CharacterParent.BP_CharacterParent_C|GetIsAlive _arrayelement)) (== (Variables|/Game/ThirdPerson/Blueprints/BP_CharacterParent.BP_CharacterParent_C|GetTeam _arrayelement) (Variables|Default|GetTeam)))
        (Utilities|Array|RemoveItem (LocalVariables|GetLcl_AllPlayer) _arrayelement)))
    (:Completed
      (if (Utilities|Array|IsNotEmpty (LocalVariables|GetLcl_AllPlayer))
        (if (== (Utilities|Array|Length (LocalVariables|GetLcl_AllPlayer)) 1)
          (LocalVariables|SetLcl_IsValidPlayerFound true)
          (LocalVariables|SetLcl_NewEnemy (Utilities|Array|Get(acopy) (LocalVariables|GetLcl_AllPlayer)))
          (return (LocalVariables|GetLcl_IsValidPlayerFound) (LocalVariables|GetLcl_NewEnemy))
          (elif FindClosestEnemy
            (bind _array_element (Utilities|Array|ForEachLoopwithBreak (LocalVariables|GetLcl_AllPlayer) :!label _label)
              (:LoopBody
                (if (< (Variables|/Game/ThirdPerson/Blueprints/BP_CharacterParent.BP_CharacterParent_C|GetNrOfAIAttacker _array_element) 4)
                  (if (< (Transformation|GetDistanceTo _array_element self) (LocalVariables|GetLcl_LowestDistance))
                    (LocalVariables|SetLcl_LowestDistance (Transformation|GetDistanceTo _array_element self))
                    (LocalVariables|SetLcl_NewEnemy _array_element)
                    (if (< (LocalVariables|GetLcl_LowestDistance) 9e+01)
                      (goto _label Break)))))
              (:Completed
                (if (> (LocalVariables|GetLcl_LowestDistance) 9.5e+03)
                  (LocalVariables|SetLcl_IsValidPlayerFound false)
                  (else
                    (LocalVariables|SetLcl_IsValidPlayerFound true)))
                (return (LocalVariables|GetLcl_IsValidPlayerFound) (LocalVariables|GetLcl_NewEnemy))))
            (else
              (for _array_element_2 (LocalVariables|GetLcl_AllPlayer)
                (Utilities|Array|Add (LocalVariables|GetLcl_AllAttackerNRs) (Variables|/Game/ThirdPerson/Blueprints/BP_CharacterParent.BP_CharacterParent_C|GetNrOfAIAttacker _array_element_2)))
              (LocalVariables|SetLcl_LowestIndex (.IndexOfMinValue (Math|Integer|MinOfIntArray (LocalVariables|GetLcl_AllAttackerNRs))))
              (if (== (LocalVariables|GetLcl_LowestIndex) -1)
                (LocalVariables|SetLcl_IsValidPlayerFound false)
                (else
                  (LocalVariables|SetLcl_NewEnemy (Utilities|Array|Get(acopy) (LocalVariables|GetLcl_AllPlayer) (LocalVariables|GetLcl_LowestIndex)))
                  (LocalVariables|SetLcl_IsValidPlayerFound true)))
              (return (LocalVariables|GetLcl_IsValidPlayerFound) (LocalVariables|GetLcl_NewEnemy)))))
        (else
          (LocalVariables|SetLcl_IsValidPlayerFound false)
          (return (LocalVariables|GetLcl_IsValidPlayerFound) (LocalVariables|GetLcl_NewEnemy)))))))

(fn GetDeathMontage
  (params (DamageDirection :type Enum_DamageDirection%20Enum :default "NewEnumerator0"))
  (switch Utilities|FlowControl|Switch|SwitchonEnum_DamageDirection DamageDirection
    (:NewEnumerator0
      _)
    (:NewEnumerator1
      _)
    (:NewEnumerator2
      _)
    (:NewEnumerator3
      _))
  (LocalVariables|SetLcl_DeathMontage "/Game/Combat/SK_Death_Montage.SK_Death_Montage")
  (return (LocalVariables|GetLcl_DeathMontage)))

(fn SetTargetPlayer
  (params (TargetPlayer :type BP%20Character%20Parent%20Object%20Reference))
  (Utilities|IsValid (Variables|Default|GetTargetPlayer)
    (:Is%20Valid
      (Math|Integer|DecrementInt (Variables|/Game/ThirdPerson/Blueprints/BP_CharacterParent.BP_CharacterParent_C|GetNrOfAIAttacker (Variables|Default|GetTargetPlayer))
        (:%20%20
          _)))
    (:Is%20Not%20Valid
      _))
  (bind _output_get (Variables|Default|SetTargetPlayer TargetPlayer))
  (Math|Integer|IncrementInt (Variables|/Game/ThirdPerson/Blueprints/BP_CharacterParent.BP_CharacterParent_C|GetNrOfAIAttacker _output_get)
    (:%20%20
      (Variables|/Game/OpenWorld/Sessions/BluePrints/GamePlay/AI/BehaviorTree/AIC_Behavior.AIC_Behavior_C|SetTargetPlayer (Variables|Default|GetAs%20AIC%20Behavior) (Variables|Default|GetTargetPlayer))
      (return))))

(fn MeleeTrace
  (bind _sword (Variables|Default|GetSword))
  (if (Variables|Default|GetCanDamageRight)
    (bind _outhit (Collision|SphereTraceForObjects (Transformation|GetSocketLocation _sword "BladeStart") (Transformation|GetSocketLocation _sword "BladeEnd") 2e+01 (Utilities|Array|MakeArray "ObjectTypeQuery3") false 0 "None" true "(R=1.000000,G=0.000000,B=0.000000,A=1.000000)" "(R=0.000000,G=1.000000,B=0.000000,A=1.000000)" 1.0))
    (if (.bBlockingHit (Collision|BreakHitResult _outhit))
      (bind _asbp_character_parent (Utilities|Casting|CastToBP_CharacterParent (.HitActor (Collision|BreakHitResult _outhit))))
      (if (!= (Variables|/Game/ThirdPerson/Blueprints/BP_CharacterParent.BP_CharacterParent_C|GetTeam _asbp_character_parent) (Variables|Default|GetTeam))
        (if (Utilities|DoesObjectImplementInterface (.HitActor (Collision|BreakHitResult _outhit)) "/Game/Combat/BPI_DamagePlayer.BPI_DamagePlayer_C")
          (Variables|Default|SetCanDamageRight false)
          (Class|BPIDamagePlayer|PlayerTakeDamage(Message) (.HitActor (Collision|BreakHitResult _outhit)) self _outhit 1e+01)
          (elif (Utilities|DoesObjectImplementInterface (.HitActor (Collision|BreakHitResult _outhit)) "/Game/OpenWorld/Sessions/BluePrints/GamePlay/AI/BPI_Damage.BPI_Damage_C")
            (Variables|Default|SetCanDamageRight false)
            (Class|BPIDamage|TakeDamage(Message) (.HitActor (Collision|BreakHitResult _outhit)) self 1e+01 (.ImpactPoint (Collision|BreakHitResult _outhit)) (.ImpactNormal (Collision|BreakHitResult _outhit)))))))))

(fn GetHitMontage
  (params (HitDirection :type Enum_DamageDirection%20Enum :default "NewEnumerator0"))
  (LocalVariables|SetLcl_GetHitMontage "/Game/Combat/SK_GetHit2.SK_GetHit2")
  (return (LocalVariables|GetLcl_GetHitMontage)))

(fn Grabbed
  (bind _returnvalue (Transformation|GetActorLocation))
  (Transformation|SetWorldLocation (Variables|Character|GetMesh) (Math|Vector|MakeVector (.x _returnvalue) (.y _returnvalue) (+ (.z _returnvalue) 2e+02)) false true)
  (return))

(fn TakeDamage
  (params (Attacker :type Actor%20Object%20Reference) (Amount :type Float%20%28double-precision%29) (Location :type Vector :default "0, 0, 0") (Normal :type Vector :default "0, 0, 0"))
  (if (Variables|Default|GetIsAlive)
    (LocalVariables|SetLcl_IsValidHit true)
    (bind _output_get (LocalVariables|SetLcl_DamageYAW (Math|Rotator|NormalizeAxis (- (.yaw (Math|Rotator|MakeRotfromZ (- (Transformation|GetActorLocation Attacker) (Transformation|GetActorLocation)))) (- (.yaw (Transformation|GetActorRotation)) (.yaw (Variables|/Script/Engine.SceneComponent|GetRelativeRotation (Variables|Character|GetMesh))))))))
    (if (< _output_get 0.0)
      (if (Math|Float|InRange(Float) (LocalVariables|GetLcl_DamageYAW) -135.0 -45.0 true false)
        (LocalVariables|SetLcl_DamageDirection "NewEnumerator0")
        (elif (>= (LocalVariables|GetLcl_DamageYAW) -45.0)
          (LocalVariables|SetLcl_DamageDirection "NewEnumerator2")
          (else
            (LocalVariables|SetLcl_DamageDirection "NewEnumerator3"))))
      (bind _output_get_2 (Variables|Default|SetHealth (- (Variables|Default|GetHealth) Amount) :!label _label))
      (if (<= _output_get_2 0.0)
        (Variables|Default|SetIsAlive false)
        (CallFunction|Die (LocalVariables|GetLcl_DamageDirection))
        (else
          (CallFunction|GetHit "/Game/Combat/SK_GetHit2.SK_GetHit2" Location Normal)))
      (return (not (Variables|Default|GetIsAlive)) (Variables|Default|GetXPWhenKilled) (LocalVariables|GetLcl_IsValidHit))
      (elif (Math|Float|InRange(Float) (LocalVariables|GetLcl_DamageYAW) 45.0 135.0 false)
        (LocalVariables|SetLcl_DamageDirection "NewEnumerator1")
        (goto _label)
        (elif (<= (LocalVariables|GetLcl_DamageYAW) 45.0)
          (LocalVariables|SetLcl_DamageDirection "NewEnumerator2")
          (else
            (LocalVariables|SetLcl_DamageDirection "NewEnumerator3")
            (goto _label)))))
    (else
      (LocalVariables|SetLcl_IsValidHit false)
      (return (not (Variables|Default|GetIsAlive)) (Variables|Default|GetXPWhenKilled) (LocalVariables|GetLcl_IsValidHit)))))