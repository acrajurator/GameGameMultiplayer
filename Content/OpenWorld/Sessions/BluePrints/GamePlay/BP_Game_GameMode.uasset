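; Game mode that handles player start, level start and death respawn for solo and multiplayer sessions.
; It tracks connected controllers and, once the Game Instance's expected count arrives (immediately if solo), places each at a PlayerStart named by array index.
; LevelStart then enables all input after short delays.
; Death respawn spawns a fresh third-person character at the indexed start, flags it DeathRespawn and possesses it.
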(event Custom|RespawnAfterDeath
  (params (PlayerController :type BP%20Game%20Player%20Controller%20Object%20Reference))
  (Pawn|UnPossess PlayerController)
  (bind _newpawn (CallFunction|RespawnPawnforController PlayerController (Class|GameModeBase|FindPlayerStart PlayerController (Utilities|String|ToString(Integer) (Utilities|Array|FindItem (Variables|Default|GetAll_ConnectedControllers) PlayerController)))))
  (Pawn|Possess PlayerController _newpawn)
  (Development|PrintString "Game Mode Possess"))

(event Custom|LevelStart
  (Utilities|FlowControl|Delay 0.2)
  (for _array_element (Variables|Default|GetAll_ConnectedControllers)
    _)
  (Utilities|FlowControl|Delay 3.0)
  (for _array_element_2 (Variables|Default|GetAll_ConnectedControllers)
    (Default|EnableAllInput _array_element_2)))

(event EventHandleStartingNewPlayer
  (params (NewPlayer :type Player%20Controller%20Object%20Reference))
  (bind _asbp_game_player_controller (Utilities|Casting|CastToBP_GamePlayerController NewPlayer))
  (Utilities|Array|Add (Variables|Default|GetAll_ConnectedControllers) _asbp_game_player_controller)
  (bind _asbp_game_game_instance (Utilities|Casting|CastToBP_Game_GameInstance (Game|GetGameInstance)))
  (Variables|Default|SetNum_ExpectedPlayers (Variables|/Game/OpenWorld/Sessions/BluePrints/GamePlay/BP_Game_GameInstance.BP_Game_GameInstance_C|GetNum%20Connected%20Players _asbp_game_game_instance))
  (if (Variables|/Game/OpenWorld/Sessions/BluePrints/GamePlay/BP_Game_GameInstance.BP_Game_GameInstance_C|GetIsSoloGame _asbp_game_game_instance)
    (Variables|Default|SetNum_ExpectedPlayers 1)
    (Class|GameModeBase|RestartPlayeratPlayerStart (Utilities|Array|Get(acopy) (Variables|Default|GetAll_ConnectedControllers)) (Class|GameModeBase|FindPlayerStart 0 "0"))
    (CallFunction|LevelStart)
    (elif (== (Variables|Default|GetNum_ExpectedPlayers) (Utilities|Array|Length (Variables|Default|GetAll_ConnectedControllers)))
      (Utilities|FlowControl|Delay 0.5)
      (for (_array_element _array_index) (Variables|Default|GetAll_ConnectedControllers)
        (Class|GameModeBase|RestartPlayeratPlayerStart _array_element (Class|GameModeBase|FindPlayerStart _array_element (Utilities|String|ToString(Integer) _array_index))))
      (CallFunction|LevelStart))))

(event EventOnLogout
  (params (ExitingController :type Controller%20Object%20Reference))
  (bind _asbp_game_player_controller (Utilities|Casting|CastToBP_GamePlayerController ExitingController))
  (Utilities|Array|RemoveItem (Variables|Default|GetAll_ConnectedControllers) _asbp_game_player_controller)
  (Math|Integer|DecrementInt (Variables|Default|GetNum_ExpectedPlayers)))

(fn ConstructionScript)

(fn RespawnPawnforController
  (params (PlayerController :type BP%20Game%20Player%20Controller%20Object%20Reference) (PlayerStart :type Actor%20Object%20Reference))
  (bind _returnvalue (Game|SpawnActorfromClass "/Game/ThirdPerson/Blueprints/BP_ThirdPersonCharacter.BP_ThirdPersonCharacter_C" (Transformation|GetActorTransform PlayerStart) "Undefined" 0 0))
  (Variables|/Game/ThirdPerson/Blueprints/BP_ThirdPersonCharacter.BP_ThirdPersonCharacter_C|SetDeathRespawn _returnvalue true)
  (return _returnvalue))