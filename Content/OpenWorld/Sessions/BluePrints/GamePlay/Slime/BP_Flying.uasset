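; BP_Flying is a temporary slime sphere effect that times out a BP_Slime owner's flying state.
; On BeginPlay it creates a dynamic slime material, then a looping timer repeatedly scales the actor up and multiplies its opacity down for a grow-and-fade look.
; A one-shot timer triggers Burst, which calls StopFlying on the owning BP_Slime and destroys the actor, provided the owner cast succeeds.
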(event Custom|Burst
  (bind _asbp_slime (Utilities|Casting|CastToBP_Slime (Components|GetOwner)))
  (Default|StopFlying _asbp_slime)
  (Actor|DestroyActor))

(event Custom|FadeAway
  (bind _self self)
  (bind _material (Variables|Default|GetMaterial))
  (Transformation|SetActorRelativeScale3D _self (* (Class|Actor|GetActorRelativeScale3D _self) 1.02))
  (bind _returnvalue (Rendering|Material|GetScalarParameterValue _material "Opacity" :!class /Script/Engine.MaterialInstanceDynamic))
  (Rendering|Material|SetScalarParameterValue _material "Opacity" (* _returnvalue 0.97) :!class /Script/Engine.MaterialInstanceDynamic))

(event EventBeginPlay
  (bind _returnvalue (Rendering|Material|CreateDynamicMaterialInstance (Variables|Default|GetSphere) 0 "/Game/OpenWorld/Sessions/BluePrints/GamePlay/Slime/MatSlime.MatSlime" "None" :!class /Script/Engine.PrimitiveComponent))
  (bind _output_get (Variables|Default|SetMaterial _returnvalue))
  (Rendering|Material|SetScalarParameterValue _output_get "Opacity" 0.9 :!class /Script/Engine.MaterialInstanceDynamic)
  (Utilities|Time|SetTimerbyEvent (delegate Custom|FadeAway) 0.1 true)
  (Utilities|Time|SetTimerbyEvent (delegate Custom|Burst) 5.0))

(event Collision|EventActorBeginOverlap
  (params (OtherActor :type Actor%20Object%20Reference)))

(event EventTick
  (params (DeltaSeconds :type Float%20%28single-precision%29)))

(fn ConstructionScript)