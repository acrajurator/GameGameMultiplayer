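; Slime projectile that damages living BP_Npc1 targets and passes its Size to any BP_Slime it hits via ChangeSize.
; Pawn collision starts as overlap and switches to block shortly after spawn.
; A looping timer then sphere-traces for pawns until the first bounce, reporting damage results to the owning slime through KillReward.
; The bullet destroys itself on a valid NPC hit or slime contact.
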(event OnProjectileBounce(ProjectileMovement)
  (params (ImpactResult :type Hit%20Result%20Structure%20%28by%20ref%29) (ImpactVelocity :type Vector%20%28by%20ref%29 :default "0, 0, 0"))
  (Utilities|Time|ClearandInvalidateTimerbyHandle (stale EventBeginPlay _returnvalue)))

(event OnComponentHit(Sphere)
  (params (HitComponent :type Primitive%20Component%20Object%20Reference) (OtherActor :type Actor%20Object%20Reference) (OtherComp :type Primitive%20Component%20Object%20Reference) (NormalImpulse :type Vector :default "0, 0, 0") (Hit :type Hit%20Result%20Structure%20%28by%20ref%29))
  (bind _asbp_slime (Utilities|Casting|CastToBP_Slime OtherActor))
  (Default|ChangeSize _asbp_slime (Variables|Default|GetSize))
  (Actor|DestroyActor))

(event Custom|BulletTrace
  (bind _isvalidhit (CallFunction|SphereTrace))
  (if _isvalidhit
    (Actor|DestroyActor)))

(event EventBeginPlay
  (Collision|SetCollisionResponsetoChannel (Variables|Default|GetSphere) "ECC_Pawn" "ECR_Overlap")
  (Utilities|FlowControl|Delay 0.1)
  (Collision|SetCollisionResponsetoChannel (Variables|Default|GetSphere) "ECC_Pawn" "ECR_Block")
  (bind _returnvalue (Utilities|Time|SetTimerbyEvent (delegate Custom|BulletTrace) 0.05 true)))

(fn ConstructionScript)

(fn SphereTrace
  (bind _returnvalue (Components|GetOwner))
  (bind _sphere (Variables|Default|GetSphere))
  (bind _returnvalue_2 (Transformation|GetWorldLocation _sphere))
  (bind (_outhit _returnvalue_3) (Collision|SphereTraceForObjects _returnvalue_2 _returnvalue_2 25.0 (Utilities|Array|MakeArray "ObjectTypeQuery3") false 0 "None"))
  (if _returnvalue_3
    (bind _asbp_npc_1 (Utilities|Casting|CastToBP_Npc1 (.HitActor (Collision|BreakHitResult _outhit))))
    (if (Variables|/Game/ThirdPerson/Blueprints/BP_CharacterParent.BP_CharacterParent_C|GetIsAlive _asbp_npc_1)
      (bind (_isdead _xp _isvalidhit) (Class|BPIDamage|TakeDamage(Message) _asbp_npc_1 _returnvalue (Variables|Default|GetDamage) (.Location (Collision|BreakHitResult _outhit)) (.Normal (Collision|BreakHitResult _outhit))))
      (bind _asbp_slime (Utilities|Casting|CastToBP_Slime _returnvalue))
      (Default|KillReward _asbp_slime _isdead _isvalidhit _xp (Utilities|GetClass _asbp_npc_1))
      (return _isvalidhit))))