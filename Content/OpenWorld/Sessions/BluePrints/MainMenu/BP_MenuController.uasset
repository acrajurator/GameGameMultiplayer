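; Menu player controller for the multiplayer lobby, handling UI-only mouse input, lobby and load-screen widgets, and leaving a session.
; InitialSetup loads or creates the saved player profile and passes it to ServerUpdateLobby, which asks BP_Menu_GameMode to refresh the lobby.
; Update events push player names and level selection into the cached lobby widget.
; Ending a client session destroys it and opens MenuLevel.
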(event Custom|EndClientSession
  (|DestroySession self
    (:then
      (Game|OpenLevel(byName) "MenuLevel"))))

(event Custom|CreateLobbyMenu
  (CallFunction|UIShowLobbyMenu))

(event Custom|InitialSetup
  (CallFunction|LoadSavedProfile)
  (CallFunction|ServerUpdateLobby (Variables|Default|GetPlayerProfileInfo)))

(event Custom|UpdatePlayerNames
  (params (PlayerProfiles :type Array%20of%20S%20Player%20Profile%20Structures))
  (bind _wb_lobbymenu (Variables|Default|GetWB_LobbyMenu)
    (:then
      (Default|ClearPlayerNames _wb_lobbymenu)
      (Default|UpdatePlayerNames _wb_lobbymenu PlayerProfiles))
    (:else)))

(event Custom|ServerUpdateLobby
  (params (PlayerProfile :type S%20Player%20Profile%20Structure))
  (Variables|Default|SetPlayerProfileInfo PlayerProfile)
  (bind _asbp_menu_game_mode (Utilities|Casting|CastToBP_Menu_GameMode (Game|GetGameMode)))
  (Default|UpdateLobby _asbp_menu_game_mode true true))

(event Custom|CreateLoadScreen
  (CallFunction|UIShowLoadScreen))

(event Custom|UpdateLevelSelection
  (params (LevelRowName :type Name))
  (bind _wb_lobbymenu (Variables|Default|GetWB_LobbyMenu)
    (:then
      (Default|UpdateLevelSelection _wb_lobbymenu LevelRowName))
    (:else)))

(event EventBeginPlay
  (if (Pawn|IsLocalController)
    (Variables|Default|SetbShowMouseCursor true)
    (Input|SetInputModeUIOnly self 0 "DoNotLock" false)))

(fn ConstructionScript)

(fn UIShowLobbyMenu
  (Variables|Default|GetWB_LobbyMenu
    (:then
      _)
    (:else
      (bind _returnvalue (UserInterface|CreateWidget "/Game/OpenWorld/Sessions/Widgets/WB_LobbyMenu.WB_LobbyMenu_C" self))
      (Variables|Default|SetWB_LobbyMenu _returnvalue)))
  (UserInterface|Viewport|AddtoViewport (Variables|Default|GetWB_LobbyMenu) 0)
  (return))

(fn LoadSavedProfile
  (bind _returnvalue (SaveGame|DoesSaveGameExist (LocalVariables|GetLcl_SlotName)))
  (if _returnvalue
    _
    (else
      (SaveGame|CreateSaveGameObject "/Game/SavedData/SG_PlayerProfile.SG_PlayerProfile_C")
      (SaveGame|SaveGametoSlot 0 (LocalVariables|GetLcl_SlotName))))
  (bind _returnvalue_2 (SaveGame|LoadGamefromSlot (LocalVariables|GetLcl_SlotName)))
  (bind _assg_player_profile (Utilities|Casting|CastToSG_PlayerProfile _returnvalue_2))
  (Variables|Default|SetPlayerProfileInfo (Variables|/Game/SavedData/SG_PlayerProfile.SG_PlayerProfile_C|GetPlayerProfile _assg_player_profile))
  (return))

(fn UIShowLoadScreen
  (Viewport|RemoveAllWidgets)
  (Variables|Default|GetWB_LoadScreen
    (:then
      _)
    (:else
      (bind _returnvalue (UserInterface|CreateWidget "/Game/OpenWorld/Sessions/Widgets/WB_LoadScreen.WB_LoadScreen_C" self))
      (Variables|Default|SetWB_LoadScreen _returnvalue)))
  (UserInterface|Viewport|AddtoViewport (Variables|Default|GetWB_LoadScreen) 0)
  (return))